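; Player controller for the horse racing game that sets the view to the TzCamera actor and manages the UI.
; BeginPlay shows the main widget and mouse cursor.
; Running-state changes swap the main widget for the ready widget on Ready, then for the game widget on Running, which is cached in the result-widget variable.
; The Finished result screen and the game-mode init and start calls are unwired.
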(event EventOnChangedRunningState
  (params (InRunningState :type ERunningState%20Enum :default "None"))
  (Utilities|FlowControl|Sequence
    (:then_0
      (if (Utilities|Enum|Equal(Enum) InRunningState "Running")
        (bind _cachedreadywidget (Variables|Default|GetCachedReadyWidget)
          (:then
            (Widget|RemovefromParent _cachedreadywidget))
          (:else
            _))
        (bind _returnvalue (UserInterface|CreateWidget "/Game/Widget/WBP_GameWidget.WBP_GameWidget_C"))
        (UserInterface|Viewport|AddtoViewport _returnvalue 0)
        (Variables|Default|SetCachedResultWidget _returnvalue)))
    (:then_1
      (if (Utilities|Enum|Equal(Enum) InRunningState "Ready")
        (bind _cachedmainwidget (Variables|Default|GetCachedMainWidget)
          (:then
            (Widget|RemovefromParent _cachedmainwidget))
          (:else
            _))
        (bind _returnvalue_2 (UserInterface|CreateWidget "/Game/Widget/WBP_ReadyWidget.WBP_ReadyWidget_C"))
        (UserInterface|Viewport|AddtoViewport _returnvalue_2 0)
        (Variables|Default|SetCachedReadyWidget _returnvalue_2)))))

(event EventTick
  (params (DeltaSeconds :type Float%20%28single-precision%29)))

(event EventBeginPlay
  (bind _returnvalue (Actor|GetActorOfClass "/Script/RunningHorse.TzCameraActor"))
  (Game|Player|SetViewTargetwithBlend _returnvalue 0.0 "VTBlend_Linear" 0.0 false)
  (bind _returnvalue_2 (UserInterface|CreateWidget "/Game/Widget/BP_MainWidget.BP_MainWidget_C"))
  (UserInterface|Viewport|AddtoViewport _returnvalue_2 0)
  (Variables|Default|SetCachedMainWidget _returnvalue_2)
  (Variables|Default|SetbShowMouseCursor true))

(fn ConstructionScript)