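; Runner game mode Blueprint that controls background music according to the game's running state.
; On BeginPlay it binds to the running-state change delegate and starts the main track, switching to the game track on Running and stopping music on Ready.
; StartBGM deactivates the current sound through StopBGM, then spawns a new 2D sound and stores it in SpawnedBGM.
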(event Custom|OnChangedRunningState
  (params (RunningState :type ERunningState%20Enum :default "None"))
  (Utilities|FlowControl|Sequence
    (:then_0
      (if (Utilities|Enum|Equal(Enum) RunningState "Running")
        (CallFunction|StartBGM (Variables|Default|GetGameBGM))))
    (:then_1
      (if (Utilities|Enum|Equal(Enum) RunningState "Ready")
        (Audio|Components|Audio|Stop (Variables|Default|GetSpawnedBGM))))))

(event EventBeginPlay
  (EventDispatchers|BindEventtoChangedRunningStateDelegate (delegate Custom|OnChangedRunningState))
  (CallFunction|StartBGM (Variables|Default|GetMainBGM)))

(event EventTick
  (params (DeltaSeconds :type Float%20%28single-precision%29)))

(fn ConstructionScript)

(fn StopBGM
  (bind _spawnedbgm (Variables|Default|GetSpawnedBGM)
    (:then
      (Components|Activation|SetActive _spawnedbgm false false))
    (:else)))

(fn StartBGM
  (params (SoundCue :type Sound%20Cue%20Object%20Reference))
  (CallFunction|StopBGM)
  (bind _returnvalue (Audio|SpawnSound2D SoundCue 1.0 1.0 0.0 0))
  (Variables|Default|SetSpawnedBGM _returnvalue))