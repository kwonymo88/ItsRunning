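; BP_ChickenRunner is a chicken runner character that takes its ranking display and color from its assigned lane.
; When OnSetupCharacterDate fires, it passes the cached lane actor's index to the BP_RankingWidget in its widget component.
; It then creates a dynamic material instance on the mesh and sets MainColor from the ColorData rank colors, treating the lane index as 1-based.
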(event EventBeginPlay)

(event Collision|EventActorBeginOverlap
  (params (OtherActor :type Actor%20Object%20Reference)))

(event EventTick
  (params (DeltaSeconds :type Float%20%28single-precision%29)))

(event EventOnSetupCharacterDate
  (bind _cachedlaneactor (Variables|Default|GetCachedLaneActor))
  (bind _returnvalue (Class|TzLane|GetLaneIndex _cachedlaneactor))
  (Utilities|FlowControl|Sequence
    (:then_0
      (bind _asbp_ranking_widget (Utilities|Casting|CastToBP_RankingWidget (UserInterface|GetWidget (Variables|Default|GetWidget))))
      (Default|SetRankingIndex _asbp_ranking_widget _returnvalue))
    (:then_1
      (CallFunction|UpdateCharacterMaterial _returnvalue))))

(fn ConstructionScript)

(fn UpdateCharacterMaterial
  (params (LaneIndex :type Integer))
  (bind _returnvalue (Rendering|Material|CreateDynamicMaterialInstance (Variables|Character|GetMesh) 0 (Rendering|Material|GetMaterial (Variables|Character|GetMesh) 0) "None" :!class /Script/Engine.PrimitiveComponent))
  (Rendering|Material|SetVectorParameterValue _returnvalue "MainColor" (Utilities|Array|Get(acopy) (Utilities|Struct|BreakFColorData (Variables|Default|GetColorData)) (- LaneIndex 1)) :!class /Script/Engine.MaterialInstanceDynamic))