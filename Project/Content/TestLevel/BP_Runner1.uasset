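; BP_Runner1 is a test-level runner character that takes its color from the lane it is assigned to.
; On the character data setup event, it reads the lane index from the cached lane actor and passes it to UpdateCharacterMaterial.
; That function creates a dynamic instance of the first mesh material and sets MainColor from the rank color data.
; The ranking widget update is left disconnected and never runs.
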(event EventBeginPlay)

(event Collision|EventActorBeginOverlap
  (params (OtherActor :type Actor%20Object%20Reference)))

(event EventTick
  (params (DeltaSeconds :type Float%20%28single-precision%29)))

(event EventOnSetupCharacterDate
  (Utilities|FlowControl|Sequence
    (:then_1
      (CallFunction|UpdateCharacterMaterial (Class|TzLane|GetLaneIndex (Variables|Default|GetCachedLaneActor))))))

(fn ConstructionScript)

(fn UpdateCharacterMaterial
  (params (LaneIndex :type Integer))
  (bind _returnvalue (Rendering|Material|CreateDynamicMaterialInstance (Variables|Character|GetMesh) 0 (Rendering|Material|GetMaterial (Variables|Character|GetMesh) 0) "None" :!class /Script/Engine.PrimitiveComponent))
  (Rendering|Material|SetVectorParameterValue _returnvalue "MainColor" (Utilities|Array|Get(acopy) (Utilities|Struct|BreakFColorData (Variables|Default|GetColorData)) (- LaneIndex 1)) :!class /Script/Engine.MaterialInstanceDynamic))