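; Test player controller that spawns and briefly plays a Niagara turtle effect when play begins.
; On BeginPlay it spawns a BP_NiagaraActor at the world origin, assigns NS_Turtle to its Niagara component at runtime and activates it.
; A one-shot timer deactivates the effect a few seconds later, leaving the spawned actor in the world.
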(event Custom|CustomEvent
  (Components|Activation|Deactivate (Variables|/Game/TestLevel/BP_NiagaraActor.BP_NiagaraActor_C|GetNiagaraSystem (Variables|Default|GetSpawnedPawn))))

(event EventBeginPlay
  (bind _returnvalue (Game|SpawnActorfromClass "/Game/TestLevel/BP_NiagaraActor.BP_NiagaraActor_C" (Math|Transform|MakeTransform "0, 0, 0") "Undefined" 0 0))
  (bind _output_get (Variables|Default|SetSpawnedPawn _returnvalue))
  (Class|NiagaraComponent|SetAsset (Variables|/Game/TestLevel/BP_NiagaraActor.BP_NiagaraActor_C|GetNiagaraSystem _output_get) "/Game/sA_PickupSet_1/Fx/NiagaraSystems/NS_Turtle.NS_Turtle" true)
  (Utilities|Time|SetTimerbyEvent (delegate Custom|CustomEvent) 3.0)
  (Components|Activation|SetActive (Variables|/Game/TestLevel/BP_NiagaraActor.BP_NiagaraActor_C|GetNiagaraSystem _output_get) true false))

(event EventTick
  (params (DeltaSeconds :type Float%20%28single-precision%29)))

(fn ConstructionScript)